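; BP_LoadoutSlot0_Component is a component for the first loadout slot that reacts when that slot is selected.
; On BeginPlay it caches the BP_GameMode reference and binds to that game mode's loadout-slot-selected event.
; The selection handler checks for the first slot enum value and currently only prints a debug message.
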(event EventBeginPlay
  ;[1 1 1] Initialise
  (CallFunction|SetReferences)
  (CallFunction|BindtoEvents))

(fn SetReferences
  ;[1 1 1] Set References
  (bind _asbp_game_mode (Utilities|Casting|CastToBP_GameMode (Game|GetGameMode)))
  (Variables|References|SetGameModeReference _asbp_game_mode))

(fn BindtoEvents
  ;[1 1 1] Bind to Events
  (EventDispatchers|BindEventtoLoadoutSlotSelected (Variables|References|GetGameModeReference) (EventDispatchers|CreateEvent :!event OnLoadoutSlotSelected)))

(fn OnLoadoutSlotSelected
  (params (LoadoutSlot :type ELoadoutSlots%20Enum :default "NewEnumerator0"))
  ;[1 1 1] Loadout Slot Selected
  (if (Utilities|Enum|Equal(Enum) LoadoutSlot "NewEnumerator0")
    (Development|PrintString "Loadout Slot 0 Selected")))