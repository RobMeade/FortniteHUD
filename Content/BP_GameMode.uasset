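; Game mode that acts as an event hub between the player controller and gameplay state such as kills, ammo, materials, loadout slots and experience.
; On BeginPlay it caches the BP_PlayerController and binds to its HUD, UI and selection events, plus change events from each stat component.
; Each handler simply re-raises the event through the game mode's own dispatchers, with HUD creation triggering a set-game-defaults event.
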(event EventBeginPlay
  ;[1 1 1] Initialise
  (CallFunction|SetReferences)
  (CallFunction|BindtoEvents))

(fn ConstructionScript)

(fn SetReferences
  ;[1 1 1] Set References
  (bind _asbp_player_controller (Utilities|Casting|CastToBP_PlayerController (Game|GetPlayerController 0)))
  (Variables|Default|SetPlayerController _asbp_player_controller))

(fn BindtoEvents
  (bind _playercontroller (Variables|Default|GetPlayerController))
  ;[1 1 1] Bind to Events
  (EventDispatchers|BindEventtoPlayerHUDCreated _playercontroller (EventDispatchers|CreateEvent :!event OnPlayerHUDCreated))
  (EventDispatchers|BindEventtoUIElementValueChanged _playercontroller (EventDispatchers|CreateEvent :!event OnUIElementValueChanged))
  (EventDispatchers|BindEventtoBuildableItemSelected _playercontroller (EventDispatchers|CreateEvent :!event OnBuildableItemSelected))
  (EventDispatchers|BindEventtoLoadoutSlotSelected _playercontroller (EventDispatchers|CreateEvent :!event OnLoadoutSlotSelected))
  (EventDispatchers|BindEventtoRemainingPlayersChanged (Variables|Default|GetRemainingPlayers) (EventDispatchers|CreateEvent :!event OnRemainingPlayersChanged))
  (EventDispatchers|BindEventtoPlayerKillsChanged (Variables|Default|GetPlayerKills) (EventDispatchers|CreateEvent :!event OnPlayerKillsChanged))
  (EventDispatchers|BindEventtoTeamKillsChanged (Variables|Default|GetTeamKills) (EventDispatchers|CreateEvent :!event OnTeamKillsChanged))
  (EventDispatchers|BindEventtoPlayerLevelChanged (Variables|Default|GetPlayerLevel) (EventDispatchers|CreateEvent :!event OnPlayerLevelChanged))
  (EventDispatchers|BindEventtoEliminationFeedChanged (Variables|Default|GetEliminationFeed) (EventDispatchers|CreateEvent :!event OnEliminationFeedChanged))
  (EventDispatchers|BindEventtoAmmoChanged (Variables|Default|GetAmmo) (EventDispatchers|CreateEvent :!event OnLoadedAmmoChanged))
  (EventDispatchers|BindEventtoMaterialsChanged (Variables|Default|GetMaterials) (EventDispatchers|CreateEvent :!event OnMaterialsChanged))
  (EventDispatchers|BindEventtoLoadoutSlot1Changed (Variables|Default|GetLoadoutSlot1) (EventDispatchers|CreateEvent :!event OnLoadoutSlot1Changed))
  (EventDispatchers|BindEventtoLoadoutSlot2Changed (Variables|Default|GetLoadoutSlot2) (EventDispatchers|CreateEvent :!event OnLoadoutSlot2Changed))
  (EventDispatchers|BindEventtoLoadoutSlot3Changed (Variables|Default|GetLoadoutSlot3) (EventDispatchers|CreateEvent :!event OnLoadoutSlot3Changed))
  (EventDispatchers|BindEventtoLoadoutSlot4Changed (Variables|Default|GetLoadoutSlot4) (EventDispatchers|CreateEvent :!event OnLoadoutSlot4Changed))
  (EventDispatchers|BindEventtoLoadoutSlot5Changed (Variables|Default|GetLoadoutSlot5) (EventDispatchers|CreateEvent :!event OnLoadoutSlot5Changed))
  (EventDispatchers|BindEventtoPlayerExperienceChanged (Variables|Default|GetPlayerExperience) (EventDispatchers|CreateEvent :!event OnPlayerExperienceChanged)))

(fn OnPlayerHUDCreated
  ;[1 1 1] Raise Event
  (Default|CallSetGameDefaults))

(fn OnUIElementValueChanged
  (params (UIElementSelection :type EUIElementTypes%20Enum :default "NewEnumerator4") (UIElementValueStep :type EUIElementValueStepTypes%20Enum :default "NewEnumerator1"))
  ;[1 1 1] Raise Event
  (Default|CallUIElementValueChanged UIElementSelection UIElementValueStep))

(fn OnRemainingPlayersChanged
  (params (Value :type Integer))
  ;[1 1 1] Raise Event
  (Default|CallRemainingPlayersChanged Value))

(fn OnPlayerKillsChanged
  (params (Value :type Integer))
  ;[1 1 1] Raise Event
  (Default|CallPlayerKillsChanged Value))

(fn OnTeamKillsChanged
  (params (Value :type Integer))
  ;[1 1 1] Raise Event
  (Default|CallTeamKillsChanged Value))

(fn OnPlayerLevelChanged
  (params (Value :type Integer))
  ;[1 1 1] Raise Event
  (Default|CallPlayerLevelChanged Value))

(fn OnEliminationFeedChanged
  (params (Value :type Array%20of%20Strings))
  ;[1 1 1] Raise Event
  (Default|CallEliminationFeedChanged Value))

(fn OnLoadedAmmoChanged
  (params (Value :type S%20Ammo%20Structure))
  ;[1 1 1] Raise Event
  (Default|CallAmmoChanged Value))

(fn OnMaterialsChanged
  (params (Value :type S%20Materials%20Structure))
  ;[1 1 1] Raise Event
  (Default|CallMaterialsChanged Value))

(fn OnBuildableItemSelected
  (params (BuildableItem :type EBuildableItems%20Enum :default "NewEnumerator0"))
  ;[1 1 1] Raise Event
  (Default|CallBuildableItemSelected BuildableItem))

(fn OnLoadoutSlot5Changed
  (params (Value :type Integer))
  ;[1 1 1] Raise Event
  (Default|CallLoadoutSlot5Changed Value))

(fn OnLoadoutSlot4Changed
  (params (Value :type Integer))
  ;[1 1 1] Raise Event
  (Default|CallLoadoutSlot4Changed Value))

(fn OnLoadoutSlot3Changed
  (params (Value :type Integer))
  ;[1 1 1] Raise Event
  (Default|CallLoadoutSlot3Changed Value))

(fn OnLoadoutSlot2Changed
  (params (Value :type Integer))
  ;[1 1 1] Raise Event
  (Default|CallLoadoutSlot2Changed Value))

(fn OnLoadoutSlot1Changed
  (params (Value :type Integer))
  ;[1 1 1] Raise Event
  (Default|CallLoadoutSlot1Changed Value))

(fn OnLoadoutSlotSelected
  (params (LoadoutSlot :type ELoadoutSlots%20Enum :default "NewEnumerator0"))
  ;[1 1 1] Raise Event
  (Default|CallLoadoutSlotSelected LoadoutSlot))

(fn OnPlayerExperienceChanged
  (params (Value :type Float%20%28single-precision%29))
  ;[1 1 1] Raise Event
  (Default|CallPlayerExperienceChanged Value))