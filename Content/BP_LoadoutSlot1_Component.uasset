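; Actor component that holds the integer setting for Loadout Slot 1 and announces changes to it.
; On BeginPlay it binds to the BP_GameMode events for setting game defaults and for UI element value changes.
; It can reset to its default, or step the value up or down by small or large amounts for its matching UI element selection.
; Steps are clamped to a minimum and maximum, and each update calls LoadoutSlot1Changed.
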(event EventBeginPlay
  ;[1 1 1] Initialise
  (CallFunction|SetReferences)
  (CallFunction|BindtoEvents))

(fn SetDefaultValue
  ;[1 1 1] Set Default Value
  (bind _output_get (Variables|Default|SetValue (Variables|Configuration|GameDefaults|GetDefaultValue)))
  (Default|CallLoadoutSlot1Changed _output_get))

(fn SetReferences
  ;[1 1 1] Set References
  (bind _asbp_game_mode (Utilities|Casting|CastToBP_GameMode (Game|GetGameMode)))
  (Variables|References|SetGameModeReference _asbp_game_mode))

(fn BindtoEvents
  (bind _gamemodereference (Variables|References|GetGameModeReference))
  ;[1 1 1] Bind to Events
  (EventDispatchers|BindEventtoSetGameDefaults _gamemodereference (EventDispatchers|CreateEvent :!event SetDefaultValue))
  (EventDispatchers|BindEventtoUIElementValueChanged _gamemodereference (EventDispatchers|CreateEvent :!event ChangeValue)))

(fn ChangeValue
  (params (UIElementSelection :type EUIElementTypes%20Enum :default "NewEnumerator4") (UIElementValueStep :type EUIElementValueStepTypes%20Enum :default "NewEnumerator1"))
  ;[1 1 1] Change Value
  (if (Utilities|Enum|Equal(Enum) UIElementSelection "NewEnumerator13")
    (switch Utilities|FlowControl|Switch|SwitchonEUIElementValueStepTypes UIElementValueStep
      (:NewEnumerator1
        (CallFunction|Decrement (Variables|Configuration|Interactivity|GetChangeStepSmall)))
      (:NewEnumerator0
        (CallFunction|Decrement (Variables|Configuration|Interactivity|GetChangeStepLarge)))
      (:NewEnumerator2
        (CallFunction|Increment (Variables|Configuration|Interactivity|GetChangeStepSmall)))
      (:NewEnumerator3
        (CallFunction|Increment (Variables|Configuration|Interactivity|GetChangeStepLarge))))))

(fn Increment
  (params (Value :type Integer))
  ;[1 1 1] Increment
  (bind _output_get (Variables|Default|SetValue (Math|Integer|Clamp(Integer) (+ (Variables|Default|GetValue) Value) (Variables|Configuration|Boundaries|GetMinimumValue) (Variables|Configuration|Boundaries|GetMaximumValue))))
  (Default|CallLoadoutSlot1Changed _output_get))

(fn Decrement
  (params (Value :type Integer))
  ;[1 1 1] Decrement
  (bind _output_get (Variables|Default|SetValue (Math|Integer|Clamp(Integer) (- (Variables|Default|GetValue) Value) (Variables|Configuration|Boundaries|GetMinimumValue) (Variables|Configuration|Boundaries|GetMaximumValue))))
  (Default|CallLoadoutSlot1Changed _output_get))