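; Storm timer component that runs a repeating countdown alternating the storm between Wait and Shrink phases.
; On BeginPlay it caches BP_GameMode, binds to its set-game-defaults event and starts a looping one-second timer for the countdown.
; When time drops below zero it resets to the default duration, shared by both phases, and toggles the mode.
; Time and mode changes are broadcast through Call events, including when defaults are applied.
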(event EventBeginPlay
  ;[1 1 1] Initialise
  (CallFunction|SetReferences)
  (CallFunction|BindtoEvents)
  (CallFunction|BeginCountdown))

(fn SetDefaultValue
  ;[1 1 1] Set Default Value
  (bind _output_get (Variables|Default|SetMode (Variables|Configuration|GameDefaults|GetDefaultMode)))
  (Default|CallStormTimerModeChanged _output_get)
  (bind _output_get_2 (Variables|Default|SetRemainingTime (Variables|Configuration|GameDefaults|GetDefaultRemainingTime)))
  (Default|CallStormTimerChanged _output_get_2))

(fn SetReferences
  ;[1 1 1] Set References
  (bind _asbp_game_mode (Utilities|Casting|CastToBP_GameMode (Game|GetGameMode)))
  (Variables|References|SetGameModeReference _asbp_game_mode))

(fn BindtoEvents
  ;[1 1 1] Bind to Events
  (EventDispatchers|BindEventtoSetGameDefaults (Variables|References|GetGameModeReference) (EventDispatchers|CreateEvent :!event SetDefaultValue)))

(fn BeginCountdown
  (Utilities|Time|SetTimerbyEvent (EventDispatchers|CreateEvent :!event OnCountdown) 1.0 true))

(fn OnCountdown
  ;[1 1 1] Countdown
  (bind _result (Math|Float|DecrementFloat (Variables|Default|GetRemainingTime))
    (:%20%20
      (if (< _result 0.0)
        (CallFunction|ResetCountdown)
        (CallFunction|ToggleStormMode)
        (else
          (Default|CallStormTimerChanged _result))))))

(fn ToggleStormMode
  ;[1 1 1] Toggle Storm Mode
  (switch Utilities|FlowControl|Switch|SwitchonEStormTimerModes (Variables|Default|GetMode)
    (:NewEnumerator0
      (Variables|Default|SetMode "NewEnumerator1"))
    (:NewEnumerator1
      (Variables|Default|SetMode "NewEnumerator0")))
  (Default|CallStormTimerModeChanged (Variables|Default|GetMode)))

(fn ResetCountdown
  ;[1 1 1] Reset Countdown
  (bind _output_get (Variables|Default|SetRemainingTime (Variables|Configuration|GameDefaults|GetDefaultRemainingTime)))
  (Default|CallStormTimerChanged _output_get))