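; Component that holds the player's Wood, Stone and Metal material counts, adjustable through UI value controls.
; On BeginPlay it caches BP_GameMode and binds to its set-game-defaults and UI-element-value-changed events.
; UI selection and step pick a small or large increment or decrement, clamped between minimum and maximum values.
; Every change, including resetting to the default, broadcasts MaterialsChanged with all three values in an SMaterials struct.
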(event EventBeginPlay
  ;[1 1 1] Initialise
  (CallFunction|SetReferences)
  (CallFunction|BindtoEvents))

(fn SetDefaultValue
  (bind _defaultvalue (Variables|Configuration|GameDefaults|GetDefaultValue))
  ;[1 1 1] Set Default Value
  (Variables|Default|SetWood _defaultvalue)
  (Variables|Default|SetStone _defaultvalue)
  (Variables|Default|SetMetal _defaultvalue)
  (Default|CallMaterialsChanged (Utilities|Struct|MakeSMaterials (Variables|Default|GetWood) (Variables|Default|GetStone) (Variables|Default|GetMetal))))

(fn SetReferences
  ;[1 1 1] Set References
  (bind _asbp_game_mode (Utilities|Casting|CastToBP_GameMode (Game|GetGameMode)))
  (Variables|References|SetGameModeReference _asbp_game_mode))

(fn BindtoEvents
  (bind _gamemodereference (Variables|References|GetGameModeReference))
  ;[1 1 1] Bind to Events
  (EventDispatchers|BindEventtoSetGameDefaults _gamemodereference (EventDispatchers|CreateEvent :!event SetDefaultValue))
  (EventDispatchers|BindEventtoUIElementValueChanged _gamemodereference (EventDispatchers|CreateEvent :!event ChangeValue)))

(fn ChangeValue
  (params (UIElementSelection :type EUIElementTypes%20Enum :default "NewEnumerator4") (UIElementValueStep :type EUIElementValueStepTypes%20Enum :default "NewEnumerator1"))
  (switch Utilities|FlowControl|Switch|SwitchonEUIElementTypes UIElementSelection
    (:NewEnumerator9
      (switch Utilities|FlowControl|Switch|SwitchonEUIElementValueStepTypes UIElementValueStep
        (:NewEnumerator1
          (CallFunction|DecrementWood (Variables|Configuration|Interactivity|GetChangeStepSmall)))
        (:NewEnumerator0
          (CallFunction|DecrementWood (Variables|Configuration|Interactivity|GetChangeStepLarge)))
        (:NewEnumerator2
          (CallFunction|IncrementWood (Variables|Configuration|Interactivity|GetChangeStepSmall)))
        (:NewEnumerator3
          (CallFunction|IncrementWood (Variables|Configuration|Interactivity|GetChangeStepLarge)))))
    (:NewEnumerator10
      (switch Utilities|FlowControl|Switch|SwitchonEUIElementValueStepTypes UIElementValueStep
        (:NewEnumerator1
          (CallFunction|DecrementStone (Variables|Configuration|Interactivity|GetChangeStepSmall)))
        (:NewEnumerator0
          (CallFunction|DecrementStone (Variables|Configuration|Interactivity|GetChangeStepLarge)))
        (:NewEnumerator2
          (CallFunction|IncrementStone (Variables|Configuration|Interactivity|GetChangeStepSmall)))
        (:NewEnumerator3
          (CallFunction|IncrementStone (Variables|Configuration|Interactivity|GetChangeStepLarge)))))
    (:NewEnumerator11
      (switch Utilities|FlowControl|Switch|SwitchonEUIElementValueStepTypes UIElementValueStep
        (:NewEnumerator1
          (CallFunction|DecrementMetal (Variables|Configuration|Interactivity|GetChangeStepSmall)))
        (:NewEnumerator0
          (CallFunction|DecrementMetal (Variables|Configuration|Interactivity|GetChangeStepLarge)))
        (:NewEnumerator2
          (CallFunction|IncrementMetal (Variables|Configuration|Interactivity|GetChangeStepSmall)))
        (:NewEnumerator3
          (CallFunction|IncrementMetal (Variables|Configuration|Interactivity|GetChangeStepLarge)))))))

(fn IncrementWood
  (params (Value :type Integer))
  ;[1 1 1] Increment
  (Variables|Default|SetWood (Math|Integer|Clamp(Integer) (+ (Variables|Default|GetWood) Value) (Variables|Configuration|Boundaries|GetMinimumValue) (Variables|Configuration|Boundaries|GetMaximumValue)))
  (Default|CallMaterialsChanged (Utilities|Struct|MakeSMaterials (Variables|Default|GetWood) (Variables|Default|GetStone) (Variables|Default|GetMetal))))

(fn DecrementWood
  (params (Value :type Integer))
  ;[1 1 1] Decrement
  (Variables|Default|SetWood (Math|Integer|Clamp(Integer) (- (Variables|Default|GetWood) Value) (Variables|Configuration|Boundaries|GetMinimumValue) (Variables|Configuration|Boundaries|GetMaximumValue)))
  (Default|CallMaterialsChanged (Utilities|Struct|MakeSMaterials (Variables|Default|GetWood) (Variables|Default|GetStone) (Variables|Default|GetMetal))))

(fn IncrementStone
  (params (Value :type Integer))
  ;[1 1 1] Increment
  (Variables|Default|SetStone (Math|Integer|Clamp(Integer) (+ (Variables|Default|GetStone) Value) (Variables|Configuration|Boundaries|GetMinimumValue) (Variables|Configuration|Boundaries|GetMaximumValue)))
  (Default|CallMaterialsChanged (Utilities|Struct|MakeSMaterials (Variables|Default|GetWood) (Variables|Default|GetStone) (Variables|Default|GetMetal))))

(fn DecrementStone
  (params (Value :type Integer))
  ;[1 1 1] Decrement
  (Variables|Default|SetStone (Math|Integer|Clamp(Integer) (- (Variables|Default|GetStone) Value) (Variables|Configuration|Boundaries|GetMinimumValue) (Variables|Configuration|Boundaries|GetMaximumValue)))
  (Default|CallMaterialsChanged (Utilities|Struct|MakeSMaterials (Variables|Default|GetWood) (Variables|Default|GetStone) (Variables|Default|GetMetal))))

(fn IncrementMetal
  (params (Value :type Integer))
  ;[1 1 1] Increment
  (Variables|Default|SetMetal (Math|Integer|Clamp(Integer) (+ (Variables|Default|GetMetal) Value) (Variables|Configuration|Boundaries|GetMinimumValue) (Variables|Configuration|Boundaries|GetMaximumValue)))
  (Default|CallMaterialsChanged (Utilities|Struct|MakeSMaterials (Variables|Default|GetWood) (Variables|Default|GetStone) (Variables|Default|GetMetal))))

(fn DecrementMetal
  (params (Value :type Integer))
  ;[1 1 1] Decrement
  (Variables|Default|SetMetal (Math|Integer|Clamp(Integer) (- (Variables|Default|GetMetal) Value) (Variables|Configuration|Boundaries|GetMinimumValue) (Variables|Configuration|Boundaries|GetMaximumValue)))
  (Default|CallMaterialsChanged (Utilities|Struct|MakeSMaterials (Variables|Default|GetWood) (Variables|Default|GetStone) (Variables|Default|GetMetal))))