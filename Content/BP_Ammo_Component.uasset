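; Ammo component that holds loaded and reserved ammo counts and broadcasts an ammo-changed event on every update.
; On BeginPlay it binds to BP_GameMode events for setting game defaults and for UI element value changes.
; UI changes map element and step type to small or large increments or decrements, clamped to each pool's minimum and maximum.
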(event EventBeginPlay
  ;[1 1 1] Initialise
  (CallFunction|SetReferences)
  (CallFunction|BindtoEvents))

(fn SetDefaultValue
  ;[1 1 1] Set Default Value
  (Variables|Default|SetLoadedValue (Variables|Configuration|GameDefaults|GetLoadedDefaultValue))
  (Variables|Default|SetReservedValue (Variables|Configuration|GameDefaults|GetReservedDefaultValue))
  (Default|CallAmmoChanged (Utilities|Struct|MakeSAmmo (Variables|Default|GetLoadedValue) (Variables|Default|GetReservedValue))))

(fn SetReferences
  ;[1 1 1] Set References
  (bind _asbp_game_mode (Utilities|Casting|CastToBP_GameMode (Game|GetGameMode)))
  (Variables|References|SetGameModeReference _asbp_game_mode))

(fn BindtoEvents
  (bind _gamemodereference (Variables|References|GetGameModeReference))
  ;[1 1 1] Bind to Events
  (EventDispatchers|BindEventtoSetGameDefaults _gamemodereference (EventDispatchers|CreateEvent :!event SetDefaultValue))
  (EventDispatchers|BindEventtoUIElementValueChanged _gamemodereference (EventDispatchers|CreateEvent :!event ChangeValue)))

(fn ChangeValue
  (params (UIElementSelection :type EUIElementTypes%20Enum :default "NewEnumerator4") (UIElementValueStep :type EUIElementValueStepTypes%20Enum :default "NewEnumerator1"))
  ;[1 1 1] Change Value
  (switch Utilities|FlowControl|Switch|SwitchonEUIElementTypes UIElementSelection
    (:NewEnumerator7
      (switch Utilities|FlowControl|Switch|SwitchonEUIElementValueStepTypes UIElementValueStep
        (:NewEnumerator1
          (CallFunction|DecrementLoaded (Variables|Configuration|Interactivity|GetLoadedChangeStepSmall)))
        (:NewEnumerator0
          (CallFunction|DecrementLoaded (Variables|Configuration|Interactivity|GetLoadedChangeStepLarge)))
        (:NewEnumerator2
          (CallFunction|IncrementLoaded (Variables|Configuration|Interactivity|GetLoadedChangeStepSmall)))
        (:NewEnumerator3
          (CallFunction|IncrementLoaded (Variables|Configuration|Interactivity|GetLoadedChangeStepLarge)))))
    (:NewEnumerator8
      (switch Utilities|FlowControl|Switch|SwitchonEUIElementValueStepTypes UIElementValueStep
        (:NewEnumerator1
          (CallFunction|DecrementReserved (Variables|Configuration|Interactivity|GetReservedChangeStepSmall)))
        (:NewEnumerator0
          (CallFunction|DecrementReserved (Variables|Configuration|Interactivity|GetReservedChangeStepLarge)))
        (:NewEnumerator2
          (CallFunction|IncrementReserved (Variables|Configuration|Interactivity|GetReservedChangeStepSmall)))
        (:NewEnumerator3
          (CallFunction|IncrementReserved (Variables|Configuration|Interactivity|GetReservedChangeStepLarge)))))))

(fn IncrementLoaded
  (params (Value :type Integer))
  ;[1 1 1] Increment
  (bind _output_get (Variables|Default|SetLoadedValue (Math|Integer|Clamp(Integer) (+ (Variables|Default|GetLoadedValue) Value) (Variables|Configuration|Boundaries|GetLoadedMinimumValue) (Variables|Configuration|Boundaries|GetLoadedMaximumValue))))
  (Default|CallAmmoChanged (Utilities|Struct|MakeSAmmo _output_get (Variables|Default|GetReservedValue))))

(fn DecrementLoaded
  (params (Value :type Integer))
  ;[1 1 1] Decrement
  (bind _output_get (Variables|Default|SetLoadedValue (Math|Integer|Clamp(Integer) (- (Variables|Default|GetLoadedValue) Value) (Variables|Configuration|Boundaries|GetLoadedMinimumValue) (Variables|Configuration|Boundaries|GetLoadedMaximumValue))))
  (Default|CallAmmoChanged (Utilities|Struct|MakeSAmmo _output_get (Variables|Default|GetReservedValue))))

(fn IncrementReserved
  (params (Value :type Integer))
  ;[1 1 1] Increment
  (bind _output_get (Variables|Default|SetReservedValue (Math|Integer|Clamp(Integer) (+ (Variables|Default|GetReservedValue) Value) (Variables|Configuration|Boundaries|GetReservedMinimumValue) (Variables|Configuration|Boundaries|GetReservedMaximumValue))))
  (Default|CallAmmoChanged (Utilities|Struct|MakeSAmmo (Variables|Default|GetLoadedValue) _output_get)))

(fn DecrementReserved
  (params (Value :type Integer))
  ;[1 1 1] Decrement
  (bind _output_get (Variables|Default|SetReservedValue (Math|Integer|Clamp(Integer) (- (Variables|Default|GetReservedValue) Value) (Variables|Configuration|Boundaries|GetReservedMinimumValue) (Variables|Configuration|Boundaries|GetReservedMaximumValue))))
  (Default|CallAmmoChanged (Utilities|Struct|MakeSAmmo (Variables|Default|GetLoadedValue) _output_get)))