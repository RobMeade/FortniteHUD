(event EventBeginPlay
  ;[1 1 1] Initialise
  (CallFunction|SetReferences)
  (CallFunction|CreateHUD)
  (CallFunction|BindtoEvents))

(event Input|ActionEvents|InputActionBuildWall
  (params (Key :type Key%20Structure :default "None"))
  ;[1 1 1] Build Menu
  (:Pressed
    (Default|CallBuildableItemSelected "NewEnumerator0")))

(event Input|ActionEvents|InputActionBuildFloor
  (params (Key :type Key%20Structure :default "None"))
  ;[1 1 1] Build Menu
  (:Pressed
    (Default|CallBuildableItemSelected "NewEnumerator1")))

(event Input|ActionEvents|InputActionLoadoutSlot0
  (params (Key :type Key%20Structure :default "None"))
  ;[1 1 1] Loadout
  (:Pressed
    (Default|CallLoadoutSlotSelected "NewEnumerator0")))

(event Input|ActionEvents|InputActionLoadoutSlot1
  (params (Key :type Key%20Structure :default "None"))
  ;[1 1 1] Loadout
  (:Pressed
    (Default|CallLoadoutSlotSelected "NewEnumerator1")))

(event Input|ActionEvents|InputActionLoadoutSlot2
  (params (Key :type Key%20Structure :default "None"))
  ;[1 1 1] Loadout
  (:Pressed
    (Default|CallLoadoutSlotSelected "NewEnumerator2")))

(event Input|ActionEvents|InputActionLoadoutSlot3
  (params (Key :type Key%20Structure :default "None"))
  ;[1 1 1] Loadout
  (:Pressed
    (Default|CallLoadoutSlotSelected "NewEnumerator3")))

(event Input|ActionEvents|InputActionLoadoutSlot4
  (params (Key :type Key%20Structure :default "None"))
  ;[1 1 1] Loadout
  (:Pressed
    (Default|CallLoadoutSlotSelected "NewEnumerator4")))

(event Input|ActionEvents|InputActionLoadoutSlot5
  (params (Key :type Key%20Structure :default "None"))
  ;[1 1 1] Loadout
  (:Pressed
    (Default|CallLoadoutSlotSelected "NewEnumerator5")))

(event Input|ActionEvents|InputActionUIToggle
  (params (Key :type Key%20Structure :default "None"))
  ;[1 1 1] Toggle UI Interactivity
  (:Pressed
    (CallFunction|ToggleUI)))

(event Input|ActionEvents|InputActionBuildSteps
  (params (Key :type Key%20Structure :default "None"))
  ;[1 1 1] Build Menu
  (:Pressed
    (Default|CallBuildableItemSelected "NewEnumerator2")))

(event Input|ActionEvents|InputActionBuildPyramid
  (params (Key :type Key%20Structure :default "None"))
  ;[1 1 1] Build Menu
  (:Pressed
    (Default|CallBuildableItemSelected "NewEnumerator3")))

(event Input|ActionEvents|InputActionBuildTrap
  (params (Key :type Key%20Structure :default "None"))
  ;[1 1 1] Build Menu
  (:Pressed
    (Default|CallBuildableItemSelected "NewEnumerator4")))

(fn ConstructionScript)

(fn SetReferences
  ;[1 1 1] Set References
  (bind _asfirst_person_character (Utilities|Casting|CastToFirstPersonCharacter (Game|GetPlayerCharacter 0)))
  (Variables|Default|SetPlayerCharacter _asfirst_person_character))

(fn CreateHUD
  (bind _self self)
  ;[1 1 1] Create HUD
  (bind _returnvalue (UserInterface|CreateWidget "/Game/WBP_HUD.WBP_HUD_C" _self))
  (bind _output_get (Variables|Default|SetHUDReference _returnvalue))
  (UserInterface|Viewport|AddtoViewport _output_get 0)
  (bind _returnvalue_2 (UserInterface|CreateWidget "/Game/WBP_HUDInteractive.WBP_HUDInteractive_C" _self))
  (bind _output_get_2 (Variables|Default|SetHUDInteractiveReference _returnvalue_2))
  (UserInterface|Viewport|AddtoViewport _output_get_2 1)
  (Widget|SetVisibility _output_get_2 "Hidden")
  (Input|SetInputModeGameOnly _self)
  (Variables|Default|SetbShowMouseCursor _self false)
  (Default|CallPlayerHUDCreated))

(fn ToggleUI
  ;[1 1 1] Toggle UI
  (Input|SetInputModeUIOnly self (Variables|Default|GetHUDReference) "DoNotLock")
  (Widget|SetVisibility (Variables|Default|GetHUDInteractiveReference) "Visible")
  (Variables|Default|SetbShowMouseCursor self true))

(fn BindtoEvents
  (bind _hudinteractivereference (Variables|Default|GetHUDInteractiveReference))
  ;[1 1 1] Bind to Events
  (EventDispatchers|BindEventtoUIElementSelectionChanged _hudinteractivereference (EventDispatchers|CreateEvent :!event OnUIElementSelectionChanged))
  (EventDispatchers|BindEventtoUIElementValueStepSelected _hudinteractivereference (EventDispatchers|CreateEvent :!event OnUIElementValueStepSelected))
  (EventDispatchers|BindEventtoCharacterRotationChanged (Variables|Default|GetPlayerCharacter) (EventDispatchers|CreateEvent :!event OnCharacterRotationChanged)))

(fn OnUIElementSelectionChanged
  (params (UIElementType :type EUIElementTypes%20Enum :default "NewEnumerator4"))
  (Variables|Default|SetUIElementSelection UIElementType))

(fn OnUIElementValueStepSelected
  (params (UIElementValueStep :type EUIElementValueStepTypes%20Enum :default "NewEnumerator1"))
  (Default|CallUIElementValueChanged (Variables|Default|GetUIElementSelection) UIElementValueStep))

(fn OnCharacterRotationChanged
  ;[1 1 1] Raise Event
  (Default|CallPlayerRotationChanged (Transformation|GetWorldRotation (Variables|/Game/FirstPersonBP/Blueprints/FirstPersonCharacter.FirstPersonCharacter_C|GetFirstPersonCamera (Variables|Default|GetPlayerCharacter)))))