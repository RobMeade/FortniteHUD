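; Component that simulates an elimination feed, generating random "eliminated ... with" messages for the UI.
; On BeginPlay it binds to BP_GameMode's defaults and UI value-change events and caches player and weapon names from data tables.
; A small increment on the matching UI element builds a random message, drops the oldest once five are held, and broadcasts the updated list through EliminationFeedChanged.
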(event EventBeginPlay
  ;[1 1 1] Initialise
  (CallFunction|SetReferences)
  (CallFunction|BindtoEvents)
  (CallFunction|GetPlayerNames)
  (CallFunction|GetWeaponNames))

(fn SetDefaultValue
  ;[1 1 1] Set Default Value
  (Utilities|Array|Clear (Variables|Default|GetEliminationFeedMessages)))

(fn SetReferences
  ;[1 1 1] Set References
  (bind _asbp_game_mode (Utilities|Casting|CastToBP_GameMode (Game|GetGameMode)))
  (Variables|References|SetGameModeReference _asbp_game_mode))

(fn BindtoEvents
  (bind _gamemodereference (Variables|References|GetGameModeReference))
  ;[1 1 1] Bind to Events
  (EventDispatchers|BindEventtoSetGameDefaults _gamemodereference (EventDispatchers|CreateEvent :!event SetDefaultValue))
  (EventDispatchers|BindEventtoUIElementValueChanged _gamemodereference (EventDispatchers|CreateEvent :!event ChangeValue)))

(fn ChangeValue
  (params (UIElementSelection :type EUIElementTypes%20Enum :default "NewEnumerator4") (UIElementValueStep :type EUIElementValueStepTypes%20Enum :default "NewEnumerator1"))
  ;[1 1 1] Change Value
  (if (Utilities|Enum|Equal(Enum) UIElementSelection "NewEnumerator6")
    (switch Utilities|FlowControl|Switch|SwitchonEUIElementValueStepTypes UIElementValueStep
      (:NewEnumerator2
        (CallFunction|DeleteMessage)
        (bind _message (CallFunction|CreateRandomMessage))
        (CallFunction|AddMessage _message)))))

(fn AddMessage
  (params (FeedMessage :type String))
  (bind _eliminationfeedmessages (Variables|Default|GetEliminationFeedMessages))
  (Utilities|Array|Add _eliminationfeedmessages FeedMessage)
  (Default|CallEliminationFeedChanged _eliminationfeedmessages))

(fn CreateRandomMessage
  (bind _playername (CallFunction|GetRandomPlayerName))
  (bind _playername_2 (CallFunction|GetRandomPlayerName))
  (bind _weaponname (CallFunction|GetRandomWeaponName))
  (return (Utilities|String|Append (Utilities|String|Append (Utilities|String|Append _playername " eliminated ") _playername_2 " with ") _weaponname)))

(fn GetRandomPlayerName
  (bind _playernames (Variables|Default|GetPlayerNames))
  (return (Utilities|Array|Get(acopy) _playernames (Math|Random|RandomIntegerinRange 0 (Utilities|Array|LastIndex _playernames)))))

(fn GetRandomWeaponName
  (bind _weaponnames (Variables|Default|GetWeaponNames))
  (return (Utilities|Array|Get(acopy) _weaponnames (Math|Random|RandomIntegerinRange 0 (Utilities|Array|LastIndex _weaponnames)))))

(fn GetPlayerNames
  (bind _outrownames (DataTable|GetDataTableRowNames "/Game/DTPlayerNames.DTPlayerNames"))
  (for _array_element _outrownames
    (bind _returnvalue (Utilities|GetDataTableRow "/Game/DTPlayerNames.DTPlayerNames" _array_element)
      (:then
        (Utilities|Array|Add (Variables|Default|GetPlayerNames) (Utilities|Struct|BreakSPlayerNames _returnvalue))))))

(fn GetWeaponNames
  (bind _outrownames (DataTable|GetDataTableRowNames "/Game/DTWeaponNames.DTWeaponNames"))
  (for _array_element _outrownames
    (bind _returnvalue (Utilities|GetDataTableRow "/Game/DTWeaponNames.DTWeaponNames" _array_element)
      (:then
        (Utilities|Array|Add (Variables|Default|GetWeaponNames) (Utilities|Struct|BreakSWeaponNames _returnvalue))))))

(fn DeleteMessage
  (if (== (Utilities|Array|Length (Variables|Default|GetEliminationFeedMessages)) 5)
    (Utilities|Array|RemoveIndex (Variables|Default|GetEliminationFeedMessages))))