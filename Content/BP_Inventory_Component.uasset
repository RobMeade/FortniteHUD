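; Inventory component that tracks an open or closed state for the inventory, with only debug output so far.
; On BeginPlay it caches the BP_GameMode reference and binds to that game mode's InventoryToggled event.
; OnInventoryToggled flips the Toggled flag and prints whether the inventory is opened or closed.
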(event EventBeginPlay
  ;[1 1 1] Initialise
  (CallFunction|SetReferences)
  (CallFunction|BindtoEvents))

(fn SetReferences
  ;[1 1 1] Set References
  (bind _asbp_game_mode (Utilities|Casting|CastToBP_GameMode (Game|GetGameMode)))
  (Variables|References|SetGameModeReference _asbp_game_mode))

(fn BindtoEvents
  ;[1 1 1] Bind to Events
  (EventDispatchers|BindEventtoInventoryToggled (Variables|References|GetGameModeReference) (EventDispatchers|CreateEvent :!event OnInventoryToggled)))

(fn OnInventoryToggled
  ;[1 1 1] Toggle Build Menu
  (bind _output_get (Variables|Default|SetToggled (not (Variables|Default|GetToggled))))
  (Development|PrintString (select _output_get "Inventory Opened" "Inventory Closed") true true "(R=0.000000,G=0.000000,B=0.000000,A=1.000000)"))