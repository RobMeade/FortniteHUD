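; BP_BuildableItems_Component listens for buildable item selections made through the game mode.
; On BeginPlay it caches a BP_GameMode reference by casting the current game mode, then binds a handler to its buildable item selected event.
; The handler currently only prints the selected enum value with a "Built" suffix, with no actual building logic.
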(event EventBeginPlay
  ;[1 1 1] Initialise
  (CallFunction|SetReferences)
  (CallFunction|BindtoEvents))

(fn SetReferences
  ;[1 1 1] Set References
  (bind _asbp_game_mode (Utilities|Casting|CastToBP_GameMode (Game|GetGameMode)))
  (Variables|References|SetGameModeReference _asbp_game_mode))

(fn BindtoEvents
  ;[1 1 1] Bind to Events
  (EventDispatchers|BindEventtoBuildableItemSelected (Variables|References|GetGameModeReference) (EventDispatchers|CreateEvent :!event OnBuildableItemSelected)))

(fn OnBuildableItemSelected
  (params (Value :type EBuildableItems%20Enum :default "NewEnumerator0"))
  ;[1 1 1] Buildable Item Selected
  (Development|PrintString (Utilities|String|Append (Utilities|String|EnumtoString Value) " Built")))